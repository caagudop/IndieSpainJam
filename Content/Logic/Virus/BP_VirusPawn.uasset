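; Virus pawn that acts as a stand-in for the mouse cursor, which it hides on BeginPlay.
; Each tick it runs a complex Visibility trace under the cursor and, on a hit, moves without sweep to the impact point, nudged back against the camera's forward vector.
; An unconnected alternative, which never runs, projects the hit onto the camera's right and up axes to hold the pawn on a plane in front of the camera.
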(event `self.ReceiveBeginPlay`
  (set `PlayerController.bShowMouseCursor` false (`GameplayStatics.GetPlayerController` 0)))

(event `self.ReceiveTick`
  (params (DeltaSeconds :type "Float (single-precision)"))
  (bind (_hitresult _returnvalue) (`PlayerController.GetHitResultUnderCursorByChannel` (`GameplayStatics.GetPlayerController` 0) "TraceTypeQuery1" true))
  (if _returnvalue
    (`self.K2_SetActorLocation` (- (`.ImpactPoint` (`GameplayStatics.BreakHitResult` _hitresult)) (* (`KismetMathLibrary.GetForwardVector` (`PlayerCameraManager.GetCameraRotation` (`GameplayStatics.GetPlayerCameraManager` 0))) 10.0)))))

(fn `UserConstructionScript`)