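; BP_Interactuable_Old is an interactable actor Blueprint that toggles a slider widget on screen with the Space Bar.
; BeginPlay creates the slider widget, adds it to the viewport hidden and keeps a reference to it.
; A FlipFlop on the key alternates between showing it with Game and UI input focused on it, and hiding it with Game Only input.
; Both branches leave the mouse cursor enabled.
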(event `self.ReceiveBeginPlay`
  (bind _returnvalue (`|CreateWidget` "/Game/Alex/BP/SliderWidget.SliderWidget_C" (`GameplayStatics.GetPlayerController` 0)))
  (bind _output_get (set `self.MySliderRef` _returnvalue))
  (`UserWidget.AddToViewport` _output_get 0)
  (`Widget.SetVisibility` (`self.MySliderRef`) "Hidden"))

(event `Key|SpaceBar`
  (params (Key :type "Key Structure"))
  (bind _returnvalue (`GameplayStatics.GetPlayerController` 0))
  (bind _mysliderref (`self.MySliderRef`))
  (:`Pressed`
    (`/Engine/EditorBlueprintResources/StandardMacros.FlipFlop`
      (:`A`
        (`Widget.SetVisibility` _mysliderref "Visible")
        (set `PlayerController.bShowMouseCursor` true _returnvalue)
        (`WidgetBlueprintLibrary.SetInputMode_GameAndUIEx` _returnvalue (`self.MySliderRef`) "LockAlways" false)
        (`KismetSystemLibrary.PrintString` "Hello"))
      (:`B`
        (`Widget.SetVisibility` _mysliderref "Hidden")
        (set `PlayerController.bShowMouseCursor` true _returnvalue)
        (`WidgetBlueprintLibrary.SetFocusToGameViewport`)
        (`WidgetBlueprintLibrary.SetInputMode_GameOnly` (`GameplayStatics.GetPlayerController` 0))))))

(fn `UserConstructionScript`)